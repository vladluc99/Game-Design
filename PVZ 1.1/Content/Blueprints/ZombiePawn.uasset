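; ZombiePawn is a simple zombie enemy pawn that walks forward and dies after taking hits.
; Each tick it teleports its location along world X by MovementSpeed, without sweeping and without scaling by delta time.
; Health starts at 100 on BeginPlay, and every hit on the Cylinder component subtracts a fixed amount.
; At zero health it destroys only the Cylinder component, leaving the actor itself alive and moving.
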(event `self.ReceiveBeginPlay`
  (set `self.Health` 100.0))

(event `self.ReceiveTick`
  (params (DeltaSeconds :type "Float (single-precision)"))
  (`self.K2_SetActorLocation` (+ (`self.K2_GetActorLocation`) (`KismetMathLibrary.MakeVector` (`self.MovementSpeed`)))))

(event `self.Cylinder.OnComponentHit`
  (params (HitComponent :type "PrimitiveComponent Object Reference") (OtherActor :type "Actor Object Reference") (OtherComp :type "PrimitiveComponent Object Reference") (NormalImpulse :type "Vector Structure") (Hit :type "HitResult Structure (by ref)"))
  (set `self.Health` (- (`self.Health`) 34.0))
  (if (<= (`self.Health`) 0.0)
    (`ActorComponent.K2_DestroyComponent` (`self.Cylinder`))))

(fn `UserConstructionScript`)